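; Player 1 controller that handles forward movement input for both local players.
; The MoveForward_p1 axis moves the controlled pawn along its control rotation's forward vector, while MoveForward_p2 does the same to Player2Ref.
; An unconnected chain that would spawn a Player 2 controller and pawn, possess it and set Player2Ref never runs, so nothing in this graph assigns that reference at runtime.
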(event `self.ReceiveBeginPlay`)

(event `InputAxis|MoveForward_p1`
  (params (AxisValue :type "Float (single-precision)"))
  (bind _returnvalue (`self.K2_GetPawn`))
  (`Pawn.AddMovementInput` _returnvalue (`KismetMathLibrary.GetForwardVector` (`Pawn.GetControlRotation` _returnvalue)) AxisValue false))

(event `InputAxis|MoveForward_p2`
  (params (AxisValue :type "Float (single-precision)"))
  (bind _player_2_ref (`self.player_2_ref`))
  (`Pawn.AddMovementInput` _player_2_ref (`KismetMathLibrary.GetForwardVector` (`Pawn.GetControlRotation` _player_2_ref)) AxisValue false))

(fn `UserConstructionScript`)